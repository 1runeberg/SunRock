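; BP_Panel is a placeable info panel with a pedestal that bobs up and down.
; The construction script gives InfoPanel a dynamic instance of M_InfoPanel_Master and applies the configured texture to its PanelTexture parameter when valid.
; Each tick, BobUpOrDown shifts Pedestal vertically by CurrentSpeed, tracks the offset in CurrentStep and reverses direction past MinMaxStep in either direction.
; The motion ignores delta time, so its rate depends on frame rate.
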(event `self.ReceiveTick`
  (params (DeltaSeconds :type "Float (single-precision)"))
  (`self.BobUpOrDown`))

(fn `BobUpOrDown`
  (bind _pedestal (`self.Pedestal`))
  (bind _currentspeed (`self.CurrentSpeed`))
  (bind (_returnvalue_x _returnvalue_y _returnvalue_z) (`KismetMathLibrary.BreakVector` (`SceneComponent.K2_GetComponentLocation` _pedestal)))
  (if (< (`self.CurrentStep`) (* (`self.MinMaxStep`) -1.0))
    (set `self.CurrentSpeed` (`KismetMathLibrary.Abs` (`self.Speed`)))
    (elif (> (`self.CurrentStep`) (`KismetMathLibrary.Abs` (`self.MinMaxStep`)))
      (set `self.CurrentSpeed` (* (`KismetMathLibrary.Abs` (`self.Speed`)) -1.0))))
  (`SceneComponent.K2_SetWorldLocation` _pedestal (`KismetMathLibrary.MakeVector` _returnvalue_x _returnvalue_y (+ _returnvalue_z _currentspeed)) false false)
  (set `self.CurrentStep` (+ (`self.CurrentStep`) _currentspeed)))

(fn `UserConstructionScript`
  (bind (_panelinfotexture_parameterinfo _panelinfotexture_parametervalue) (break `TextureParameterValue` (`self.PanelInfoTexture`)))
  (bind _returnvalue (`KismetMaterialLibrary.CreateDynamicMaterialInstance` "/Game/SunRock/MaterialLibrary/InfoPanels/M_InfoPanel_Master.M_InfoPanel_Master"))
  (`PrimitiveComponent.SetMaterial` (`self.InfoPanel`) 0 _returnvalue)
  (if (`KismetSystemLibrary.IsValid` _panelinfotexture_parametervalue)
    (`MaterialInstanceDynamic.SetTextureParameterValue` _returnvalue "PanelTexture" _panelinfotexture_parametervalue)))